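; BP_BaseEnemy is a base enemy that destroys itself when a player throws a bomb.
; On BeginPlay it binds to the ThrowBomb event of each BP_ThirdPersonCharacter player.
; A MoveToPlayer event uses AI Move To on player 0, but its only call here is disconnected.
; Closest-player targeting is unfinished: the distance check is disconnected and the FindClosest and GetPlayerPosition events are empty.
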(event `self.ReceiveBeginPlay`
  ;[1 1 1] BombStuff Dylan
  (bind _outactors (`GameplayStatics.GetAllActorsOfClass` "/Game/ThirdPerson/Blueprints/BP_ThirdPersonCharacter.BP_ThirdPersonCharacter_C"))
  (for _index (range (+ (`KismetArrayLibrary.Array_Length` _outactors) 1))
    (bind _asbp_third_person_character (cast `/Game/ThirdPerson/Blueprints/BP_ThirdPersonCharacter` (`GameplayStatics.GetPlayerCharacter` _index)))
    (add `/Game/ThirdPerson/Blueprints/BP_ThirdPersonCharacter.ThrowBomb` _asbp_third_person_character (delegate `BombThrown`))))

(event `BombThrown`
  ;[1 1 1] BombStuff Dylan
  (if true
    (`self.K2_DestroyActor`)))

(event `MoveToPlayer`
  ;[1 1 1 1 14] DT - BaseEnemy Movement
  (bind _outactors (`GameplayStatics.GetAllActorsOfClass` "/Game/ThirdPerson/Blueprints/BP_ThirdPersonCharacter.BP_ThirdPersonCharacter_C"))
  (bind _output_get (set `self.TargetPlayer` (`|GetArrayItem` _outactors)))
  (for (_array_element _array_index) _outactors
    (bind _asbp_third_person_character (cast `/Game/ThirdPerson/Blueprints/BP_ThirdPersonCharacter` (`GameplayStatics.GetPlayerCharacter` 0)))
    (bind _output_get_2 (set `self.Player REF` _asbp_third_person_character))
    (`|AIMoveTo` self (`self.PlayerPOS`) _output_get_2)))

(event `FindClosest`)

(event `GetPlayerPosition`)

(fn `UserConstructionScript`)